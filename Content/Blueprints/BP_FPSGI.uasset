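; BP_FPSGI is the game instance that carries the first-person character's inventory across level changes.
; OpenLevelWithItems saves the Inventory component's item classes and current item index, then opens the named level.
; RestorePlayerInventory spawns a fresh actor for each saved class, gives it to the player character and reselects the saved index.
; Only classes and the selected index are saved, not per-item state.
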(fn `OpenLevelWithItems`
  (params (LevelName :type Name))
  (bind _asbp_first_person_character (cast `/Game/Blueprints/BP_FirstPersonCharacter` (`GameplayStatics.GetPlayerCharacter` 0)))
  (bind _inventory (`/Game/Blueprints/BP_FirstPersonCharacter.Inventory` _asbp_first_person_character))
  (set `self.SavedPlayerInventory` (`InventoryComponent.GetItemsClasses` _inventory))
  (set `self.CurrentItemIndex` (`InventoryComponent.GetCurrentItemIndex` _inventory))
  (`GameplayStatics.OpenLevel` LevelName))

(fn `RestorePlayerInventory`
  (bind _savedplayerinventory (`self.SavedPlayerInventory`))
  (if (> (`KismetArrayLibrary.Array_Length` _savedplayerinventory) 0)
    (for _array_element _savedplayerinventory
      (bind _returnvalue (`|SpawnActorFromClass` _array_element (`KismetMathLibrary.MakeTransform` (0.0 0.0 0.0)) "AlwaysSpawn" "OverrideRootScale" null null))
      (`PickupableItem.GiveItem` _returnvalue (`GameplayStatics.GetPlayerCharacter` 0)))
    (bind _asbp_first_person_character (cast `/Game/Blueprints/BP_FirstPersonCharacter` (`GameplayStatics.GetPlayerCharacter` 0)))
    (`InventoryComponent.SelectItem` (`/Game/Blueprints/BP_FirstPersonCharacter.Inventory` _asbp_first_person_character) (`self.CurrentItemIndex`))))