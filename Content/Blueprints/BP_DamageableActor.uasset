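; BP_DamageableActor is a damageable static mesh actor that takes hits, shows damage popups and is destroyed when its health runs out.
; GetDamage subtracts damage from Health and spawns a WB_DmgPop widget with the rounded value at the hit location projected to screen.
; A surviving actor returns true and, if its mesh simulates physics, receives the hit impulse at that location.
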(fn `GetDamage`
  (params (Damage :type "Float (double-precision)") (Impulse :type "Vector Structure") (Location :type "Vector Structure"))
  (returns (Success :type Boolean))
  (bind _staticmesh (`self.StaticMesh`))
  (set `self.Health` (- (`self.Health`) Damage))
  (bind _returnvalue (`|CreateWidget` "/Game/Blueprints/Widgets/WB_DmgPop.WB_DmgPop_C" null (`GameplayStatics.ProjectWorldToScreen` (`GameplayStatics.GetPlayerController` 0) Location) (`KismetMathLibrary.Round` Damage)))
  (`UserWidget.AddToViewport` _returnvalue 0)
  (if (<= (`self.Health`) 0.0)
    (`self.K2_DestroyActor`)
    (else
      (if (`SceneComponent.IsSimulatingPhysics` _staticmesh "None")
        (`PrimitiveComponent.AddImpulseAtLocation` _staticmesh Impulse Location "None"))
      (return true))))

(fn `UserConstructionScript`)