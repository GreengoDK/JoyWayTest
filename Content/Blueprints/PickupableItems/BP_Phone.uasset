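; BP_Phone is a pickupable phone item with a WB_Phone screen widget, attached to the character's left-hand grip when given.
; BeginPlay caches the widget and plays its Fade animation forward.
; Interacting shows the mouse cursor and reverses the fade.
; Tick watches for the phone being hidden while the cursor shows, then hides the cursor, restores game-only input and replays the forward fade.
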(event `self.ReceiveBeginPlay`
  (bind _phonewidget (`self.PhoneWidget`))
  (bind _aswb_phone (cast `/Game/Blueprints/Widgets/WB_Phone` (`WidgetComponent.GetUserWidgetObject` (`self.Widget`))))
  (set `self.PhoneWidget` _aswb_phone)
  (`UserWidget.PlayAnimationForward` _phonewidget (`/Game/Blueprints/Widgets/WB_Phone.Fade` _phonewidget) 1.0 false :!label _label))

(event `self.ReceiveTick`
  (params (DeltaSeconds :type "Float (single-precision)"))
  (bind _returnvalue (`GameplayStatics.GetPlayerController` 0))
  (`parent.ReceiveTick` DeltaSeconds)
  (if (`PlayerController.bShowMouseCursor` (`GameplayStatics.GetPlayerController` 0))
    (if (`self.bHidden`)
      (set `PlayerController.bShowMouseCursor` false _returnvalue)
      (`WidgetBlueprintLibrary.SetInputMode_GameOnly` _returnvalue)
      (goto _label))))

(fn `GiveItem`
  (params (ReceivingPawn :type "Pawn Object Reference"))
  (returns (ReturnValue :type Boolean))
  (bind _returnvalue (`parent.GiveItem` ReceivingPawn))
  (`self.K2_AttachToComponent` (`/Game/Blueprints/BP_FirstPersonCharacter.FirstPersonMesh` (`self.Character`)) "GripPointLeft" "SnapToTarget" "SnapToTarget" "KeepWorld")
  (return _returnvalue))

(fn `OnInteractPressed`
  (returns (Result :type Boolean))
  (bind _returnvalue (`GameplayStatics.GetPlayerController` 0))
  (bind _phonewidget (`self.PhoneWidget`))
  (if (not (`PlayerController.bShowMouseCursor` _returnvalue))
    (set `PlayerController.bShowMouseCursor` true _returnvalue)
    (`UserWidget.PlayAnimationReverse` _phonewidget (`/Game/Blueprints/Widgets/WB_Phone.Fade` _phonewidget) 1.0 false)
    (return true)))

(fn `UserConstructionScript`
  (`parent.UserConstructionScript`))