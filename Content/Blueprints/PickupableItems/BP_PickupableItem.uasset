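; Base pickup item Blueprint that spins in the world until a first-person character receives it.
; Tick yaws the CollisionVolume a fixed step each frame while the item is not Equipped.
; GiveItem casts the receiver to BP_FirstPersonCharacter, adds itself to that Inventory, snaps to the first-person mesh's GripPoint socket and sets Equipped.
; Interact press and release handlers are stubs that return false.
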(event `self.ReceiveTick`
  (params (DeltaSeconds :type "Float (single-precision)"))
  (if (not (`self.Equipped`))
    (`SceneComponent.K2_AddWorldRotation` (`self.CollisionVolume`) (struct :`Yaw` 1.2) false false)))

(fn `GiveItem`
  (params (ReceivingPawn :type "Pawn Object Reference"))
  (returns (ReturnValue :type Boolean))
  (bind _asbp_first_person_character (cast `/Game/Blueprints/BP_FirstPersonCharacter` ReceivingPawn))
  (set `self.Character` _asbp_first_person_character)
  (`InventoryComponent.AddItem` (`/Game/Blueprints/BP_FirstPersonCharacter.Inventory` _asbp_first_person_character) self)
  (`self.K2_AttachToComponent` (`/Game/Blueprints/BP_FirstPersonCharacter.FirstPersonMesh` _asbp_first_person_character) "GripPoint" "SnapToTarget" "SnapToTarget" "KeepWorld")
  (set `self.Equipped` true)
  (return true))

(fn `OnInteractPressed`
  (returns (Result :type Boolean))
  (return false))

(fn `OnInteractReleased`
  (returns (Result :type Boolean))
  (return false))

(fn `UserConstructionScript`)