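; BP_RifleLaser is a pickupable laser rifle that fires a continuous damaging beam while the interact input is held.
; Press and release toggle the beam and impact effects; Tick also releases it when the rifle is hidden.
; While enabled, Tick line-traces from the Ammo socket along the camera's forward direction, sending random damage and an impulse to the hit actor.
; The trace sets the beam's end parameter and moves or toggles the impact emitter.
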(event `self.ReceiveBeginPlay`)

(event `self.ReceiveTick`
  (params (DeltaSeconds :type "Float (single-precision)"))
  (`parent.ReceiveTick` DeltaSeconds)
  (if (`self.bHidden`)
    (`self.OnInteractReleased`)
    (elif (`self.LaserEnabled`)
      (`self.UpdateEmmitersAndApplyDamage`))))

(fn `OnInteractPressed`
  (returns (Result :type Boolean))
  (set `self.LaserEnabled` true)
  (`ActorComponent.Activate` (`self.Laser`) false)
  (`ActorComponent.Activate` (`self.E_Laser_System`) false)
  (return false))

(fn `OnInteractReleased`
  (returns (Result :type Boolean))
  (set `self.LaserEnabled` false)
  (`ActorComponent.Deactivate` (`self.Laser`))
  (`ActorComponent.Deactivate` (`self.E_Laser_System`))
  (return false))

(fn `UpdateEmmitersAndApplyDamage`
  (bind _e_laser_system (`self.E_Laser_System`))
  (bind _laser (`self.Laser`))
  (bind _returnvalue (`SceneComponent.GetSocketLocation` (`self.SkeletalMesh`) "Ammo"))
  (bind _returnvalue_2 (`ActorComponent.IsActive` _e_laser_system))
  (bind _returnvalue_3 (+ _returnvalue (* (`KismetMathLibrary.GetForwardVector` (`PlayerCameraManager.GetCameraRotation` (`GameplayStatics.GetPlayerCameraManager` 0))) 5000.0)))
  (bind (_outhit _returnvalue_4) (`KismetSystemLibrary.LineTraceSingle` _returnvalue _returnvalue_3 "TraceTypeQuery1" true))
  (if _returnvalue_4
    (bind (_bblockinghit _binitialoverlap _time _distance _location _impactpoint _normal _impactnormal _physmat _hitactor) (`GameplayStatics.BreakHitResult` _outhit))
    (message `/Game/Blueprints/IDamageable.GetDamage` _hitactor (`KismetMathLibrary.RandomFloatInRange` 0.1 2.0) (- _location _returnvalue) _location)
    (`FXSystemComponent.SetVectorParameter` _laser "LaserEnd" _location)
    (`SceneComponent.K2_SetWorldLocation` (`self.E_Laser_System`) _location false false)
    (if (not _returnvalue_2)
      (`ActorComponent.Activate` _e_laser_system true))
    (else
      (`FXSystemComponent.SetVectorParameter` _laser "LaserEnd" _returnvalue_3)
      (if _returnvalue_2
        (`ActorComponent.Deactivate` _e_laser_system)))))

(fn `UserConstructionScript`
  (`parent.UserConstructionScript`))